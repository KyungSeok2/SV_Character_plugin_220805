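; BP_PlayerStat holds a player's stats in the Propnight play level: HP, death count, rescue count and collected map pieces.
; Damage and heal functions clamp HP, and damage that empties it increments the death count unless the Death flag is set.
; RepNotify functions broadcast HP, death and rescue changes through event dispatchers, with the two counts intended for the GameState.
; Debug prints report deaths and HP updates.
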(fn ConstructionScript)

(fn AddDamageAddDeathCount
  (params (Damage :type Float%20%28single-precision%29))
  ;[1 1 1] 데미지를 전달 받으면
  ; 데미지 수치만큼 HP값을 뺀다
  (bind _output_get (Variables|Default|SetHP (Math|Float|Clamp(Float) (- (Variables|Default|GetHP) Damage) 0.0 1e+02)))
  ;[1 1 1] HP가
  (if (and (<= _output_get 0.0) (not (Variables|Default|GetDeath?)))
    (bind _output_get_2 (Variables|Default|SetDeathCount (+ (Variables|Default|GetDeathCount) 1)))
    (Development|PrintString (Utilities|String|Append "death" (Utilities|String|ToString(Integer) _output_get_2)) true true "(R=1.000000,G=0.057403,B=0.000000,A=1.000000)" 5.0)))

(fn AddHeal
  (params (Heal :type Float%20%28single-precision%29))
  (Variables|Default|SetHP (Math|Float|Clamp(Float) (+ (Variables|Default|GetHP) Heal) 0.0 1e+02)))

(fn OnRepHP
  (bind _hp (Variables|Default|GetHP))
  (Development|PrintString (Utilities|String|Append "OnRepHP - " (Utilities|String|ToString(Float) _hp)) true true "(R=0.000000,G=0.660000,B=1.000000,A=1.000000)" 6e+01)
  (Default|CallEventDispatcherHP _hp 1e+02))

(fn IsDeath
  ;[1 1 1] 코멘트
  (if (<= (Variables|Default|GetHP) 0.0)
    (return true)
    (else
      (return false))))

(fn AddMapPiece
  (Variables|Default|SetMapPiece (+ (Variables|Default|GetMapPiece) 1)))

(fn AddRescueCount
  (Variables|Default|SetRescueCount (+ (Variables|Default|GetRescueCount) 1)))

(fn OnRepRescueCount
  ;[1 1 1] 게임스테이트로 카운트 값 전달
  (Default|CallEventDispatcherRescueCount (Variables|Default|GetRescueCount)))

(fn OnRepDeathCount
  ;[1 1 1] 게임스테이트로 카운트 값 전달
  (Default|CallEventDispatcherDeathCount (Variables|Default|GetDeathCount)))
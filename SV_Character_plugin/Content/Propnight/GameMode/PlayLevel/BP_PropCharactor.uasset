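; Survivor's prop-disguise pawn for Propnight: a physics-simulated static mesh moved by forces and jump impulses.
; Left click traces from the camera to copy a "prop"-tagged actor's mesh and material; right click or death repossesses the linked BP_SurvivorCharacter.
; Possession changes toggle mesh visibility, collision and physics, while Tick relays mesh and spring arm transforms through server events.
; Damage accumulates in BP_PlayerStat, playing a hit sound or triggering death; debug keys remain.
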(event OnComponentHit(StaticMesh)
  (params (HitComponent :type Primitive%20Component%20Object%20Reference) (OtherActor :type Actor%20Object%20Reference) (OtherComp :type Primitive%20Component%20Object%20Reference) (NormalImpulse :type Vector :default "0, 0, 0") (Hit :type Hit%20Result%20Structure%20%28by%20ref%29))
  ;[1 1 1 1 70] 점프
  (Utilities|IsValid OtherActor
    (:Is%20Valid
      (Variables|Default|SetIsGround true))
    (:Is%20Not%20Valid
      (Variables|Default|SetIsGround false))))

(event Custom|req_test
  (bind _my_survivor_character (Variables|Default|GetMy%20Survivor%20Character))
  ;[0.1823 0.1823 0.1823] 코멘트
  (Utilities|IsValid _my_survivor_character
    (:Is%20Valid
      (Development|PrintString (Utilities|String|Append (Utilities|GetDisplayName _my_survivor_character) " / " (Utilities|GetObjectName _my_survivor_character)) true true "(R=0.000000,G=0.660000,B=1.000000,A=1.000000)" 5.0))
    (:Is%20Not%20Valid
      (Development|PrintString "None" true true "(R=1.000000,G=0.000000,B=0.000000,A=1.000000)" 5.0))))

(event Custom|req_death
  (bind _self self)
  (bind _returnvalue (Transformation|GetActorLocation _self))
  ;[1 1 1] 코멘트
  ;;[1 1 1 1 70] 현재 캐릭터의 빙의를 풀고 원래 캐릭터로 빙의 (우클릭)
  ;;;[1 0 0] 서버에서 이벤트 실행
  (Transformation|SetActorLocation (Variables|Default|GetMy%20Survivor%20Character) (Math|Vector|MakeVector (.x _returnvalue) (.y _returnvalue) (+ (.z _returnvalue) 1e+02)) false false)
  (Utilities|FlowControl|Delay 0.4)
  ;;;;[0 1 1] 빙의해제 -> 다른캐릭터에 빙의
  (Pawn|Possess (Pawn|GetController) (Variables|Default|GetMy%20Survivor%20Character)))

(event Custom|res_to%20human_Server
  (bind _self self)
  (bind _returnvalue (Transformation|GetActorLocation _self))
  ;[1 1 1] 코멘트
  ;;[1 1 1 1 70] 현재 캐릭터의 빙의를 풀고 원래 캐릭터로 빙의 (우클릭)
  ;;;[1 0 0] 서버에서 이벤트 실행
  (Transformation|SetActorLocation (Variables|Default|GetMy%20Survivor%20Character) (Math|Vector|MakeVector (.x _returnvalue) (.y _returnvalue) (+ (.z _returnvalue) 1e+02)) false false)
  (Utilities|FlowControl|Delay 0.4)
  ;;;;[0 1 1] 빙의해제 -> 다른캐릭터에 빙의
  (Pawn|Possess (Pawn|GetController) (Variables|Default|GetMy%20Survivor%20Character)))

(event Custom|req_Server%20Loc%20Rot
  (params (Static%20Mesh :type Static%20Mesh%20Component%20Object%20Reference) (Mesh%20Location :type Vector) (Mesh%20Rotation :type Rotator) (Spring%20Arm :type Spring%20Arm%20Component%20Object%20Reference) (Spring%20Arm%20Rotation :type Rotator))
  ;[1 1 1 1 70] Tick) 서버에 캐릭터의 위치값 회전값 전달
  ;;[1 0 0] (서버->클라)
  (CallFunction|ResServerLocRot Static%20Mesh Mesh%20Location Mesh%20Rotation Spring%20Arm Spring%20Arm%20Rotation))

(event Custom|res_Server%20Loc%20Rot
  (params (Static%20Mesh :type Static%20Mesh%20Component%20Object%20Reference) (Mesh%20Location :type Vector) (Mesh%20Rotation :type Rotator) (Spring%20Arm :type Spring%20Arm%20Component%20Object%20Reference) (Spring%20Arm%20Rotation :type Rotator))
  ;[1 1 1 1 70] Tick) 서버에 캐릭터의 위치값 회전값 전달
  ;;[1 1 1] 전달받은 위치값을 각 클라이언트에 업데이트
  (Transformation|SetWorldLocationAndRotation Static%20Mesh Mesh%20Location Mesh%20Rotation false false)
  (Transformation|SetWorldRotation Spring%20Arm Spring%20Arm%20Rotation false false))

(event Custom|커스텀이벤트_0
  ;[0 0 0 1 70] 프랍_ 굴리기(폐기)
)

(event Custom|res_Add%20Damage
  ;[1 1 1] 맞는소리
  (Audio|PlaySoundatLocation "/SV_Character_plugin/Propnight/Audio/Damage_Cue.Damage_Cue" (Transformation|GetWorldLocation (Variables|Default|GetStatic%20Mesh)) "0, 0, 0" 1.0 1.0 0.0 0 0 0))

(event Custom|req_transform
  (bind _camera (Variables|Default|GetCamera))
  (bind _returnvalue (Transformation|GetWorldLocation _camera))
  (bind _returnvalue_2 (Math|Vector|GetForwardVector _camera))
  ;[1 1 1] 코멘트
  ;;[1 1 1 1 70] 다른 프롭으로 변신 (좌클릭)
  ;;;[1 0 0] 클라->서버)
  ;;;;[1 1 1] 카메라 보는 방향으로 라인트레이스 발사
  (bind _outhit (Collision|LineTraceByChannel (+ _returnvalue (* _returnvalue_2 700)) (+ _returnvalue (* _returnvalue_2 1200)) "TraceTypeQuery1" false 0 "ForDuration"))
  ;;;;[1 1 1] 대상이 Prop 태그를 가지고 있다면
  (Utilities|IsValid (.hitactor _outhit)
    (:Is%20Valid
      (if (Actor|ActorHasTag (.hitactor _outhit) "prop")
        ;;;;[1 1 1] 스테틱매시 컴포넌트를 추출해서 클라이언트에 전달
        (CallFunction|ResTransform (Variables|/Script/Engine.StaticMeshComponent|GetStaticMesh (Actor|GetComponentbyClass (.hitactor _outhit) "/Script/Engine.StaticMeshComponent")) (Rendering|Material|GetMaterial (Variables|/Script/Engine.StaticMeshComponent|GetStaticMesh (Actor|GetComponentbyClass (.hitactor _outhit) "/Script/Engine.StaticMeshComponent")) 0))))))

(event Custom|res_transform
  (params (Static%20Mesh :type Static%20Mesh%20Object%20Reference) (Material%20Interface :type Material%20Interface%20Object%20Reference))
  ;[1 1 1] 코멘트
  ;;[1 1 1 1 70] 다른 프롭으로 변신 (좌클릭)
  ;;;[1 1 1] 서버에서 전달받은 스테틱매시, 머터리얼로 변경
  (CallFunction|PRSetStaticMesh Static%20Mesh Material%20Interface))

(event Custom|Test
  ;[0.224 0.224 0.224] 테스트 데미지
  (Game|Damage|ApplyDamage self 4e+01 0 0))

(event Custom|res_Client%20Possess
  (bind _static_mesh (Variables|Default|GetStatic%20Mesh))
  ;[1 1 1] 코멘트
  ;;[1 1 1 1 70] 빙의 될때 이벤트
  ;;;[1 1 1] 보이기
  (Variables|Default|SetPossess true)
  (Rendering|SetVisibility _static_mesh true false)
  (Collision|SetCollisionEnabled _static_mesh "QueryAndPhysics")
  (Physics|SetSimulatePhysics _static_mesh true)
  (Collision|SetCollisionResponsetoChannel (Variables|Default|GetStatic%20Mesh) "ECC_Pawn" "ECR_Block"))

(event Custom|res_Client%20UnPossess
  (bind _static_mesh (Variables|Default|GetStatic%20Mesh))
  ;[1 1 1] 코멘트
  ;;[1 1 1 1 70] 빙의 풀렸을때 이벤트
  ;;;[1 1 1] 숨기기
  (Variables|Default|SetPossess false)
  (Rendering|SetVisibility _static_mesh false false)
  (Physics|SetSimulatePhysics _static_mesh false)
  (Collision|SetCollisionEnabled _static_mesh "NoCollision")
  (Collision|SetCollisionResponsetoChannel (Variables|Default|GetStatic%20Mesh) "ECC_Pawn" "ECR_Ignore"))

(event EventPossessed
  (params (NewController :type Controller%20Object%20Reference))
  ;[1 1 1] 코멘트
  ;;[1 1 1 1 70] 빙의 될때 이벤트
  ;;;[1 0 0] (서버->클라)
  (CallFunction|ResClientPossess))

(event EventUnpossessed
  (params (OldController :type Controller%20Object%20Reference))
  ;[1 1 1] 코멘트
  ;;[1 1 1 1 70] 빙의 풀렸을때 이벤트
  ;;;[1 0 0] (서버->클라)
  (CallFunction|ResClientUnPossess))

(event EventSetCharacter
  (params (SurvivorCharacter :type Character%20Object%20Reference))
  ;[1 1 1 1 70] 스폰이벤트
  (bind _asbp_survivor_character (Utilities|Casting|CastToBP_SurvivorCharacter SurvivorCharacter)
    (:then
      (Variables|Default|SetMy%20Survivor%20Character _asbp_survivor_character))
    (:CastFailed
      (Development|PrintString "SurvivorCharacter Cast Failed" true true "(R=1.000000,G=0.000000,B=0.062734,A=1.000000)"))))

(event EventTick
  (params (DeltaSeconds :type Float%20%28single-precision%29))
  (bind _springarm (Variables|Default|GetSpringArm))
  (bind _static_mesh (Variables|Default|GetStatic%20Mesh))
  (bind _relativerotation (Variables|/Script/Engine.SceneComponent|GetRelativeRotation _springarm))
  ;[1 1 1 1 70] Tick) 서버에 캐릭터의 위치값 회전값 전달
  ;;[1 1 1] SpringArm의 회전값을
  ;; 컨트롤러의 Y,Z 값으로 설정되며 X는 0으로 고정
  (Transformation|AddRelativeRotation _springarm (Math|Rotator|MakeRotator 0.0 (Class|Actor|GetInputAxisKeyValue) (Class|Actor|GetInputAxisKeyValue)) false false)
  ;;[1 1 1] SpringArm의 pitch값 제한
  (Transformation|SetRelativeRotation _springarm (Math|Rotator|MakeRotator (.roll _relativerotation) (Math|Float|ClampAngle (.pitch _relativerotation) -25.0 4e+01) (.yaw _relativerotation)) false false)
  ;;[1 1 1] 서버에 PropCharactor, SpringArm의 위치값, 회전값 전달
  (CallFunction|ReqServerLocRot _static_mesh (Transformation|GetWorldLocation _static_mesh) (Transformation|GetWorldRotation _static_mesh) _springarm (Transformation|GetWorldRotation _springarm)))

(event Game|Damage|EventAnyDamage
  (params (Damage :type Float%20%28single-precision%29) (DamageType :type Damage%20Type%20Object%20Reference) (InstigatedBy :type Controller%20Object%20Reference) (DamageCauser :type Actor%20Object%20Reference))
  ;[1 0 0] 데미지 이벤트
  (bind _asbp_player_stat (Utilities|Casting|CastToBP_PlayerStat (Variables|GetPlayerState)))
  (if (not (Default|IsDeath _asbp_player_stat))
    (Default|AddDamageAddDeathCount _asbp_player_stat Damage)
    (if (Default|IsDeath _asbp_player_stat)
      (Variables|/SV_Character_plugin/Propnight/GameMode/PlayLevel/BP_PlayerStat.BP_PlayerStat_C|SetDeath? _asbp_player_stat true)
      ;;[1 1 1] 빙의해제이벤트로 전달
      (CallFunction|ReqDeath)
      (bind _asbp_survivor_character (Utilities|Casting|CastToBP_SurvivorCharacter (Variables|Default|GetMy%20Survivor%20Character)))
      ;;[1 1 1] 캐릭터의 사망 이벤트
      (Default|ResDeath _asbp_survivor_character)
      (else
        ;[1 1 1] 맞는소리
        (CallFunction|ResAddDamage)))))

(event Input|ActionEvents|InputActionJump
  (params (Key :type Key%20Structure))
  ;[1 1 1 1 70] 점프
  (:Pressed
    (if (Variables|Default|GetIsGround)
      (Variables|Default|SetIsGround false)
      (Physics|AddImpulseatLocation (Variables|Default|GetStatic%20Mesh) "0, 0,40000.000000" (Transformation|GetWorldLocation (Variables|Default|GetStatic%20Mesh)) "None")))
  (:Released
    (Variables|Default|SetIsGround false)))

(event Input|AxisEvents|InputAxisMoveForward
  (params (AxisValue :type Float%20%28single-precision%29))
  (bind _springarm (Variables|Default|GetSpringArm))
  (bind _relativerotation (Variables|/Script/Engine.SceneComponent|GetRelativeRotation _springarm))
  ;[1 1 1 1 70] 이동 (WASD)
  (if (Physics|IsSimulatingPhysics (Variables|Default|GetStatic%20Mesh) "None")
    (Physics|AddForce (Variables|Default|GetStatic%20Mesh) (* (Math|Vector|GetForwardVector (Math|Rotator|MakeRotator (.roll _relativerotation) 0.0 (.yaw _relativerotation))) (* AxisValue 1.5e+03)) "None" true)))

(event Input|AxisEvents|InputAxisMoveRight
  (params (AxisValue :type Float%20%28single-precision%29))
  (bind _springarm (Variables|Default|GetSpringArm))
  (bind _relativerotation (Variables|/Script/Engine.SceneComponent|GetRelativeRotation _springarm))
  ;[1 1 1 1 70] 이동 (WASD)
  (if (Physics|IsSimulatingPhysics (Variables|Default|GetStatic%20Mesh) "None")
    (Physics|AddForce (Variables|Default|GetStatic%20Mesh) (* (Math|Vector|GetRightVector (Math|Rotator|MakeRotator (.roll _relativerotation) 0.0 (.yaw _relativerotation))) (* AxisValue 1.5e+03)) "None" true)))

(event Input|KeyboardEvents|E
  (params (Key :type Key%20Structure))
  (bind _springarm (Variables|Default|GetSpringArm))
  (bind _returnvalue (Transformation|GetWorldRotation _springarm))
  ;[0.1823 0.1823 0.1823] 코멘트
  (:Pressed
    (Transformation|SetWorldRotation (Variables|Default|GetStatic%20Mesh) "0, 0, 0" false false)
    (Pawn|SetControlRotation (Pawn|GetController) (Math|Rotator|MakeRotator (.roll _returnvalue) (.pitch _returnvalue) (.yaw _returnvalue)))
    (Development|PrintString (Utilities|String|ToString(Float) (.yaw _returnvalue)))))

(event Input|MouseEvents|LeftMouseButton
  (params (Key :type Key%20Structure))
  ;[1 1 1] 코멘트
  ;;[1 1 1 1 70] 다른 프롭으로 변신 (좌클릭)
  ;;;[1 1 1] 다른 프롭으로 변신(클라->서버)
  (:Pressed
    (CallFunction|ReqTransform)))

(event Input|MouseEvents|RightMouseButton
  (params (Key :type Key%20Structure))
  ;[1 1 1] 코멘트
  ;;[1 1 1 1 70] 현재 캐릭터의 빙의를 풀고 원래 캐릭터로 빙의 (우클릭)
  ;;;[1 1 1] 변신 해제
  (:Pressed
    (Transformation|SetWorldRotation (Variables|Default|GetStatic%20Mesh) "0, 0, 0" false false)
    (Pawn|SetControlRotation (Pawn|GetController) (Transformation|GetWorldRotation (Variables|Default|GetSpringArm)))
    (CallFunction|RestoHumanServer)))

(event Input|KeyboardEvents|3
  (params (Key :type Key%20Structure))
  ;[0.224 0.224 0.224] 테스트 데미지
  (:Pressed
    (CallFunction|Test)))

(event Input|KeyboardEvents|Q
  (params (Key :type Key%20Structure))
  ;[1 1 1 1 70] 위치 정렬 (Q키)
  (:Pressed
    (Transformation|SetRelativeRotation (Variables|Default|GetStatic%20Mesh) (Math|Rotator|MakeRotator 0.0 0.0 (.yaw (Variables|/Script/Engine.SceneComponent|GetRelativeRotation (Variables|Default|GetSpringArm)))) false false)))

(event Input|KeyboardEvents|2
  (params (Key :type Key%20Structure))
  ;[0.1823 0.1823 0.1823] 코멘트
  (:Pressed
    (CallFunction|ReqTest)))

(fn ConstructionScript)

(fn PRSetStaticMesh
  (params (GetStaticMesh :type Static%20Mesh%20Object%20Reference) (GetMaterial :type Material%20Interface%20Object%20Reference) (SurvivorCharacter :type Character%20Object%20Reference))
  ;[1 1 1] SurvivorCharacter 혹은
  ; PropCharacter 에서
  ; 상호작용키(F) 누를때 함수 실행
  ;[1 1 1] 스테틱매시를 가져온다.
  (Components|StaticMesh|SetStaticMesh (Variables|Default|GetStatic%20Mesh) GetStaticMesh)
  (Rendering|Material|SetMaterial (Variables|Default|GetStatic%20Mesh) 0 GetMaterial)
  ;[1 1 1] 매쉬의 콜리젼 상태 확인 후
  ; (콜리전상태 == 빙의상태)
  (if (not (Class|PrimitiveComponent|IsCollisionEnabled (Variables|Default|GetStatic%20Mesh)))
    ;[1 1 1] 콜리젼이 꺼져있으면 SpringArm의 회전값을
    ; SurvivorCharacter의 회전값으로 설정한다.
    (Transformation|SetRelativeRotation (Variables|Default|GetSpringArm) (Pawn|GetControlRotation SurvivorCharacter :!class /Script/Engine.Pawn) false false)))

(fn OnRepPitch)

(fn PRDie)